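; BP_CANON is an automatic cannon that repeatedly fires BP_Projectile actors from its Arrow component's location and rotation.
; Tick enters a Delay set by CanonFireRate, then spawns a projectile scaled by CannonProjectileScale.
; The FIRE timeline then animates the Canon component's relative Y position with each shot, and its Finished output loops back into the Delay.
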(event `self.ReceiveTick`
  (params (DeltaSeconds :type "Float (single-precision)"))
  (bind _arrow (`self.Arrow`))
  (`KismetSystemLibrary.Delay` (`self.Canon Fire Rate`) :!label _label)
  (`|SpawnActorFromClass` "/Game/Blueprints/BP_Projectile.BP_Projectile_C" (`KismetMathLibrary.MakeTransform` (`SceneComponent.K2_GetComponentLocation` _arrow) (`SceneComponent.K2_GetComponentRotation` _arrow) (`KismetMathLibrary.Conv_DoubleToVector` (`self.Cannon ProjectileScale`))) "Undefined" "OverrideRootScale" null null)
  (bind (_direction _fired) (`Timeline|FIRE` :!via `PlayFromStart`)
    (:`Update`
      (`SceneComponent.K2_SetRelativeLocation` (`self.canon`) (`KismetMathLibrary.MakeVector` 0.0 _fired) false false))
    (:`Finished`
      (goto _label))))

(fn `UserConstructionScript`)