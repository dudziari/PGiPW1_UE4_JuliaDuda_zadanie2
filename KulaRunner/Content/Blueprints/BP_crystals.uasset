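; BP_crystals is a pickup crystal that flies into the player and vanishes when the player's pawn overlaps its trigger.
; The overlap plays a 2D sound, then after a short delay starts the MovementCrystal timeline.
; Each update lerps from the current location and scale toward the pawn's live position and zero size, so the crystal homes in while shrinking.
; The timeline also drives the light's intensity, and the actor destroys itself when it finishes.
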(event `self.triggerek.OnComponentBeginOverlap`
  (params (OverlappedComponent :type "PrimitiveComponent Object Reference") (OtherActor :type "Actor Object Reference") (OtherComp :type "PrimitiveComponent Object Reference") (OtherBodyIndex :type Integer) (bFromSweep :type Boolean) (SweepResult :type "HitResult Structure (by ref)"))
  (if (== OtherActor (`GameplayStatics.GetPlayerPawn` 0))
    ;[1 0.6249 0.08374] Sound
    (`GameplayStatics.SpawnSound2D` "/Game/Blueprints/503492__larakaa__yumyum__1_.503492__larakaa__yumyum__1_" 1.0 1.0 0.0 null)
    (`KismetSystemLibrary.Delay` 0.2)
    ;[0.3543 0.8079 1] Animation
    (bind (_direction _crytsal_movement _crystal_scale _crystal_light) (`Timeline|movement crystal`)
      (:`Update`
        (`self.K2_SetActorLocation` (`KismetMathLibrary.VLerp` (`self.K2_GetActorLocation`) (`self.K2_GetActorLocation` (`GameplayStatics.GetPlayerPawn` 0)) _crytsal_movement))
        ;;[0.5205 0.207 1] Animation - Scale
        (`self.SetActorScale3D` (`KismetMathLibrary.VLerp` (`self.GetActorScale3D`) (0.0 0.0 0.0) _crystal_scale))
        ;;[0.5136 1 0.1932] Animation - Blinking
        (`LightComponent.SetIntensity` (`self.crystal light`) (`KismetMathLibrary.Lerp` 1000.0 0.0 _crystal_light)))
      (:`Finished`
        (`self.K2_DestroyActor`)))))

(fn `UserConstructionScript`)